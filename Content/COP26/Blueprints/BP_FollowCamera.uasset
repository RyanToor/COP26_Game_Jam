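; Follow camera actor that tracks FollowActor's height, holding its starting X and Y and flooring Z to whole units.
; On BeginPlay it creates a scaled, rotated Paper2D background sprite component.
; Each Tick it offsets active background sprites by minus half a scene component's world Z for vertical parallax.
; When FollowActor enters a new 1280-unit vertical chunk, it calls CheckChunks on GM_Level and stores the chunk index.
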(event `self.ReceiveBeginPlay`
  (bind (_returnvalue_x _returnvalue_y) (`KismetMathLibrary.BreakVector` (`self.K2_GetActorLocation` self)))
  (set `self.StartX` _returnvalue_x)
  (set `self.StartY` _returnvalue_y)
  (bind _returnvalue (`AddComponent|NODE_AddPaperSpriteComponent-0` :`RelativeTransform` (`KismetMathLibrary.MakeTransform` (`KismetMathLibrary.MakeVector` (`self.BackgroundYDisplacement`)) (struct :`Yaw` -90.0))))
  (`SceneComponent.SetWorldScale3D` _returnvalue (2.0 2.0 2.0))
  (`KismetArrayLibrary.Array_Add` (`self.BackgroundSprites`) _returnvalue)
  (`KismetArrayLibrary.Array_Add` (`self.BackgroundSprites_Active`) _returnvalue))

(event `self.ReceiveTick`
  (params (DeltaSeconds :type "Float (single-precision)"))
  (bind (_returnvalue_x _returnvalue_y _returnvalue_z) (`KismetMathLibrary.BreakVector` (`self.K2_GetActorLocation` (`self.FollowActor`))))
  (bind (_returnvalue_x_2 _returnvalue_y_2 _returnvalue_z_2) (`KismetMathLibrary.BreakVector` (`SceneComponent.K2_GetComponentLocation` (`self.SceneComponent`))))
  (bind _returnvalue (`KismetMathLibrary.Abs_Int` (`KismetMathLibrary.FTrunc` (/ _returnvalue_z 1280.0))))
  (`self.K2_SetActorLocation` (`KismetMathLibrary.MakeVector` (`self.StartX`) (`self.StartY`) (`KismetMathLibrary.Conv_IntToDouble` (`KismetMathLibrary.FFloor` _returnvalue_z))))
  (for _array_element (`self.BackgroundSprites_Active`)
    (`SceneComponent.K2_SetRelativeLocation` _array_element (`KismetMathLibrary.MakeVector` (`self.BackgroundYDisplacement`) _returnvalue_x_2 (* _returnvalue_z_2 -0.5)) false false))
  (if (!= _returnvalue (`self.CurrentChunk`))
    (`/Game/COP26/Framework/GM_Level.CheckChunks` (cast `/Game/COP26/Framework/GM_Level` (`GameplayStatics.GetGameMode`) :!pure true) _returnvalue)
    (set `self.CurrentChunk` _returnvalue)))

(fn `UserConstructionScript`)