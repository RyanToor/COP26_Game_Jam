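; BP_RandomTrash is a drifting trash prop that shows a configurable Paper2D sprite tumbling as it moves.
; The construction script sets the sprite, random starting rotation and random spin speed from a min/max range.
; It also builds an InterpToMovement path that swings to both ends along X, shifted by Start, and returns to origin over Duration.
; Tick advances the sprite's pitch using delta time for frame-rate-independent spin.
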(event `self.ReceiveTick`
  (params (DeltaSeconds :type "Float (single-precision)"))
  (bind _returnvalue (`KismetMathLibrary.ComposeRotators` (`self.Rotation`) (`KismetMathLibrary.MakeRotator` 0.0 (* (`self.FrameRotation`) (`GameplayStatics.GetWorldDeltaSeconds`)))))
  (`SceneComponent.K2_SetRelativeRotation` (`self.PaperSprite`) _returnvalue false false)
  (set `self.Rotation` _returnvalue))

(fn `UserConstructionScript`
  (bind _interptomovement (`self.InterpToMovement`))
  (`PaperSpriteComponent.SetSprite` (`self.PaperSprite`) (`self.Sprite`))
  (set `InterpToMovementComponent.ControlPoints` (`|MakeArray` (make `InterpControlPoint` (0.0 0.0 0.0)) (make `InterpControlPoint` (`KismetMathLibrary.MakeVector` (- 1000.0 (`self.Start`)))) (make `InterpControlPoint` (`KismetMathLibrary.MakeVector` (- -1000.0 (`self.Start`)))) (make `InterpControlPoint` (0.0 0.0 0.0))) _interptomovement)
  (set `InterpToMovementComponent.Duration` (`self.Duration`) _interptomovement)
  (set `self.Rotation` (`KismetMathLibrary.MakeRotator` 0.0 (* (`KismetMathLibrary.RandomFloat`) 360.0)))
  (set `self.FrameRotation` (+ (`self.MinFrameRotation`) (`KismetMathLibrary.RandomFloatInRange` (`self.MinFrameRotation`) (`self.MaxFrameRotation`)))))