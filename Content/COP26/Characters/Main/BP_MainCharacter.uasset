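; Player character for a side-view Paper2D swimming game that collects trash and takes damage from obstacle trash.
; Overlaps either raise the trash count or apply knockback and damage, updating the PC_Level UI widgets.
; Zero health pauses the game, shows GameOver and saves the high score.
; Tick tilts the body by velocity, drives swim/idle flipbooks through a transition, and switches from Flying to Falling above a fixed height.
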(event `self.ReceiveBeginPlay`
  (`GameplayStatics.PlaySound2D` "/Game/COP26/Audio/Music/BackgroundSound_Cue.BackgroundSound_Cue" 1.0 1.0 0.0 null null))

(event `self.ReceiveActorBeginOverlap`
  (params (OtherActor :type "Actor Object Reference"))
  (bind _currenttrash (`self.currentTrash`))
  (bind _highscoresave (`self.HighScoreSave`))
  (bind _asbp_random_trash_collectable (cast `/Game/COP26/Blueprints/BP_RandomTrash_Collectable` OtherActor)
    (:`then`
      (bind _result (`/Engine/EditorBlueprintResources/StandardMacros.IncrementInt` (`self.currentTrash`))
        (:`  `
          (`GameplayStatics.PlaySound2D` "/Game/COP26/Audio/SFX/CollectablesSound_Cue.CollectablesSound_Cue" 1.0 1.0 0.0 null null)
          (`self.K2_DestroyActor` _asbp_random_trash_collectable)
          (set `/Game/COP26/UI/Trash_Hunt_UI.currentTrash` _result (`/Game/COP26/Framework/PC_Level.WBP_UI` (cast `/Game/COP26/Framework/PC_Level` (`GameplayStatics.GetPlayerController` 0) :!pure true))))))
    (:`CastFailed`
      (bind _asbp_random_trash (cast `/Game/COP26/Blueprints/BP_RandomTrash` OtherActor))
      (set `MovementComponent.Velocity` (* (`KismetMathLibrary.Normal` (- (`SceneComponent.K2_GetComponentLocation` (`self.CapsuleComponent`)) (`SceneComponent.K2_GetComponentLocation` (`/Game/COP26/Blueprints/BP_RandomTrash.PaperSprite` _asbp_random_trash)))) (/ (`/Game/COP26/Blueprints/BP_RandomTrash.KnockbackForce` _asbp_random_trash) (`/Game/COP26/Blueprints/BP_RandomTrash.Duration` _asbp_random_trash))) (`self.CharacterMovement`))
      (`self.K2_DestroyActor` _asbp_random_trash)
      (`GameplayStatics.PlaySound2D` "/Game/COP26/Audio/SFX/ObstacleHit_Cue.ObstacleHit_Cue" 1.0 1.0 0.0 null null)
      (bind _output_get (set `self.Health` (- (`self.Health`) (`self.Damage`))))
      (set `/Game/COP26/UI/Health_UI.Health` _output_get (`/Game/COP26/Framework/PC_Level.WBP_Health` (cast `/Game/COP26/Framework/PC_Level` (`GameplayStatics.GetPlayerController` 0) :!pure true)))
      (if (== (`self.Health`) 0)
        (`self.K2_DestroyActor`)
        (`GameplayStatics.SetGamePaused` true)
        (bind _returnvalue (`|CreateWidget` "/Game/COP26/UI/GameOver.GameOver_C"))
        (`UserWidget.AddToViewport` _returnvalue 0)
        (set `PlayerController.bShowMouseCursor` true (`GameplayStatics.GetPlayerController` 0))
        (bind _returnvalue_2 (`GameplayStatics.DoesSaveGameExist` "ScoreData"))
        (if _returnvalue_2
          (bind _returnvalue_3 (`GameplayStatics.LoadGameFromSlot` "ScoreData"))
          (bind _output_get_2 (set `self.HighScoreSave` _returnvalue_3))
          (bind _ashigh_score_save_game (cast `/Game/COP26/Framework/HighScoreSaveGame` _output_get_2))
          (if (> _currenttrash (`/Game/COP26/Framework/HighScoreSaveGame.HighScore` _ashigh_score_save_game))
            (set `/Game/COP26/Framework/HighScoreSaveGame.HighScore` _currenttrash _ashigh_score_save_game)
            (`GameplayStatics.SaveGameToSlot` _highscoresave "ScoreData"))
          (else
            (bind _returnvalue_4 (`GameplayStatics.CreateSaveGameObject` "/Game/COP26/Framework/HighScoreSaveGame.HighScoreSaveGame_C"))
            (bind _output_get_3 (set `self.HighScoreSave` _returnvalue_4))
            (bind _ashigh_score_save_game_2 (cast `/Game/COP26/Framework/HighScoreSaveGame` _output_get_3))
            (set `/Game/COP26/Framework/HighScoreSaveGame.HighScore` _currenttrash _ashigh_score_save_game_2)
            (`GameplayStatics.SaveGameToSlot` _highscoresave "ScoreData")))))))

(event `InputAxis|MoveUp`
  (params (AxisValue :type "Float (single-precision)"))
  (`self.AddMovementInput` (0.0 0.0 1.0) AxisValue))

(event `InputAxis|MoveRight`
  (params (AxisValue :type "Float (single-precision)"))
  (`self.AddMovementInput` (1.0 0.0 0.0) AxisValue)
  (bind _output_get (set `self.MovementInput` AxisValue))
  (if (> _output_get 0.0)
    (set `self.bIsMovingRight` true)
    (elif (< _output_get 0.0)
      (set `self.bIsMovingRight` false))))

(event `self.ReceiveTick`
  (params (DeltaSeconds :type "Float (single-precision)"))
  (bind _charactermovement (`self.CharacterMovement`))
  (bind (_returnvalue_x _returnvalue_y _returnvalue_z) (`KismetMathLibrary.BreakVector` (`SceneComponent.K2_GetComponentLocation` (`self.CapsuleComponent`))))
  (bind _maxflyspeed (`CharacterMovementComponent.MaxFlySpeed` _charactermovement))
  (bind _velocity (`MovementComponent.Velocity` _charactermovement))
  (bind _returnvalue (`KismetMathLibrary.Lerp` -90.0 90.0 (+ (/ (/ (.z _velocity) _maxflyspeed) 2.0) 0.5)))
  (`PaperFlipbookComponent.SetPlayRate` (`self.Sprite`) (`KismetMathLibrary.Lerp` 0.2 1.5 (/ (`KismetMathLibrary.VSize` _velocity) _maxflyspeed)))
  (`/Engine/EditorBlueprintResources/StandardMacros.CompareFloat` (`self.MovementInput`)
    (:`>`
      (set `self.TargetRotation` (`KismetMathLibrary.MakeRotator` 180.0 (* _returnvalue -1.0) 180.0) :!label _label))
    (:`==`
      (if (`self.bisMovingRight`)
        (goto _label)
        (else
          (set `self.TargetRotation` (`KismetMathLibrary.MakeRotator` 0.0 _returnvalue 180.0) :!label _label_2))))
    (:`<`
      (goto _label_2)))
  (`SceneComponent.K2_SetWorldRotation` (`self.CapsuleComponent`) (`KismetMathLibrary.ComposeRotators` (`KismetMathLibrary.RInterpTo` (`SceneComponent.K2_GetComponentRotation` (`self.Sprite`)) (`self.TargetRotation`) (`GameplayStatics.GetWorldDeltaSeconds`)) (struct :`Pitch` 90.0)) false false)
  (`self.UpdateAnimation`)
  (`CharacterMovementComponent.SetMovementMode` (`self.CharacterMovement`) (select `bool` (> _returnvalue_z -100.0) :`false` "MOVE_Flying" :`true` "MOVE_Falling" :!type "EMovementMode Enum") 0))

(event `UpdateAnimation`
  (bind _sprite (`self.Sprite`))
  (bind _sprite_2 (`self.Sprite`))
  (bind _returnvalue (`PaperFlipbookComponent.GetPlaybackPositionInFrames` _sprite_2))
  (bind _returnvalue_2 (`KismetSystemLibrary.GetDisplayName` (`PaperFlipbookComponent.GetFlipbook` (`self.Sprite`))))
  (bind _returnvalue_3 (> (`KismetMathLibrary.VSize` (`MovementComponent.Velocity` (`self.CharacterMovement`))) 0.0))
  (if (`KismetStringLibrary.EqualEqual_StrStr` _returnvalue_2 "PF_Idle")
    (if _returnvalue_3
      (`PaperFlipbookComponent.SetFlipbook` _sprite "/Game/COP26/Characters/Main/PF_Transition_Swim-Idle.PF_Transition_Swim-Idle")
      (`PaperFlipbookComponent.SetPlayRate` _sprite -1.0)
      (`PaperFlipbookComponent.SetLooping` _sprite true :!label _label_3))
    (elif (`KismetStringLibrary.EqualEqual_StrStr` _returnvalue_2 "PF_Swim")
      (if (not _returnvalue_3)
        (`PaperFlipbookComponent.SetFlipbook` _sprite "/Game/COP26/Characters/Main/PF_Transition_Swim-Idle.PF_Transition_Swim-Idle")
        (`PaperFlipbookComponent.SetPlayRate` _sprite 1.0)
        (goto _label_3))
      (elif (`KismetStringLibrary.EqualEqual_StrStr` _returnvalue_2 "PF_Transition_Swim-Idle")
        (if (or (== (`PaperFlipbook.GetNumFrames` (`PaperFlipbookComponent.GetFlipbook` _sprite_2)) _returnvalue) (== _returnvalue 0))
          (`PaperFlipbookComponent.SetFlipbook` (`self.Sprite`) (select `bool` (> (`KismetMathLibrary.VSize` (`MovementComponent.Velocity` (`self.CharacterMovement`))) 0.0) :`false` "/Game/COP26/Characters/Main/PF_Idle.PF_Idle" :`true` "/Game/COP26/Characters/Main/PF_Swim.PF_Swim" :!type "PaperFlipbook Object Reference")))))))

(fn `UserConstructionScript`)