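; Level game mode that builds an endless, descending chasm from chunks as CheckChunks receives the current index.
; Random seeds drive each BP_Chunk, with chasm width adjusted linearly by depth.
; It keeps the current chunk and its neighbours visible, generating missing ones and hiding the rest without destroying them.
; Each new chunk also spawns trash, with count and odds of dangerous rather than collectable pieces scaling with depth.
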(event `self.ReceiveBeginPlay`
  (bind _output_get (set `self.PerlinSeeds` (make `IntPoint` (`KismetMathLibrary.RandomInteger` 10000) (`KismetMathLibrary.RandomInteger` 10000))))
  (`KismetSystemLibrary.PrintString` (`KismetStringLibrary.Conv_IntPointToString` _output_get) true true (struct :`G` 0.66 :`B` 1.0 :`A` 1.0) 5.0)
  (`self.CheckChunks` 0))

(event `CheckChunks`
  (params (ChunkIndex :type Integer))
  (bind _returnvalue (- ChunkIndex 1))
  (bind _returnvalue_2 (+ ChunkIndex 1))
  (for _index (range _returnvalue (+ _returnvalue_2 1))
    (if (>= _index 0)
      (if (`KismetArrayLibrary.Array_IsValidIndex` (`self.Chunks`) _index)
        (`self.Activate/DeactivateChunk` _index)
        (else
          (`self.GenerateChunk` _index)))))
  (for (_ _array_index) (`self.Chunks`)
    (if (not (or (== _array_index _returnvalue) (== _array_index ChunkIndex) (== _array_index _returnvalue_2)))
      (`self.Activate/DeactivateChunk` _array_index true))))

(fn `Activate/DeactivateChunk`
  (params (ChunkIndex :type Integer) (Disabled :type Boolean))
  (`self.SetActorHiddenInGame` (`|GetArrayItem` (`self.Chunks`) ChunkIndex) Disabled))

(fn `GenerateChunk`
  (params (MapIndex :type Integer))
  (bind _returnvalue (`KismetMathLibrary.RandomFloatInRange` 5.0 10.0))
  (bind _returnvalue_2 (`KismetMathLibrary.RandomFloatInRange` -100.0 100.0))
  (bind _chasmwidthdecrease (`self.ChasmWidthDecrease`))
  (bind _returnvalue_3 (`KismetMathLibrary.Conv_IntToDouble` (- (* MapIndex -1280) (`KismetMathLibrary.RandomInteger` 1279))))
  (bind _returnvalue_4 (`|SpawnActorFromClass` "/Game/Individual_Folders/Ryan/BP_Chunk.BP_Chunk_C" (`KismetMathLibrary.MakeTransform` (0.0 0.0 0.0)) "Undefined" "OverrideRootScale" self (`self.PerlinSeeds`) MapIndex (- (`self.ChasmStartWidth`) (* MapIndex _chasmwidthdecrease)) _chasmwidthdecrease null))
  (`KismetArrayLibrary.Array_Insert` (`self.Chunks`) _returnvalue_4 MapIndex)
  (`KismetArrayLibrary.Array_Insert` (`self.ActiveChunks`) _returnvalue_4 MapIndex)
  (for _ (range 1 (+ (`KismetMathLibrary.FCeil` (/ (`KismetMathLibrary.Conv_IntToDouble` MapIndex) (`KismetMathLibrary.Conv_IntToDouble` (`self.Trash IncreaseLevels`)))) 1))
    (if (< (`KismetMathLibrary.RandomInteger` 100) (* MapIndex (`self.DangerSpawnChance`)))
      (`|SpawnActorFromClass` "/Game/Individual_Folders/Pacome/RandomTrashGenerator/RandomTrash.RandomTrash_C" (`KismetMathLibrary.MakeTransform` (`KismetMathLibrary.MakeVector` _returnvalue_2 -10.0 _returnvalue_3)) "Undefined" "OverrideRootScale" null _returnvalue _returnvalue_2 null)
      (else
        (`|SpawnActorFromClass` "/Game/Individual_Folders/Pacome/RandomTrashGenerator/RandomTrash_Collectable.RandomTrash_Collectable_C" (`KismetMathLibrary.MakeTransform` (`KismetMathLibrary.MakeVector` _returnvalue_2 -10.0 _returnvalue_3)) "Undefined" "OverrideRootScale" null _returnvalue _returnvalue_2 null))))
  (return))

(fn `UserConstructionScript`)