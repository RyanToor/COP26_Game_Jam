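; PC_Level is the player controller for a COP26 level with a trash hunt UI.
; On BeginPlay it creates the Trash_Hunt_UI widget, adds it to the viewport and sets game-only input.
; SetWidgetImage creates a WBP_TestMapRT widget on first use, then assigns the passed image to one of its two brushes based on the map index.
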(event `self.ReceiveBeginPlay`
  (bind _returnvalue (`|CreateWidget` "/Game/COP26/UI/Trash_Hunt_UI.Trash_Hunt_UI_C" self))
  (bind _output_get (set `self.WBP_UI` _returnvalue))
  (`UserWidget.AddToViewport` _output_get 0)
  (`WidgetBlueprintLibrary.SetInputMode_GameOnly` self))

(event `SetWidgetImage`
  (params (Image :type "SlateBrush Structure") (MapIndex :type Integer))
  (bind _wbp_test (`self.WBP_Test`))
  (`/Engine/EditorBlueprintResources/StandardMacros.IsValid` (`self.WBP_Test`)
    (:`Is Valid`
      _)
    (:`Is Not Valid`
      (bind _returnvalue (`|CreateWidget` "/Game/Individual_Folders/Ryan/WBP_TestMapRT.WBP_TestMapRT_C" self))
      (bind _output_get (set `self.WBP_Test` _returnvalue))
      (`UserWidget.AddToViewport` _output_get 0)))
  (switch `int` MapIndex
    (:`0`
      (set `/Game/Individual_Folders/Ryan/WBP_TestMapRT.SlateBrush_1` Image _wbp_test))
    (:`1`
      (set `/Game/Individual_Folders/Ryan/WBP_TestMapRT.SlateBrush_2` Image _wbp_test))))

(fn `UserConstructionScript`)