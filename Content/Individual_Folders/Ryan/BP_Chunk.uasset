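; BP_Chunk procedurally generates one 30x20 Paper2D tilemap section of a vertical chasm, stacked downward by ChunkIndex.
; On BeginPlay, seeded 1D Perlin noise sets each row's left and right wall thickness, which is recorded in Maps.
; Adjacent chunks' edge rows are computed as padding, letting DetermineTile pick edge, corner and fill tiles that match across seams.
; PlaceTiles paints both walls, then collision is rebuilt to block Pawns.
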(event `self.ReceiveBeginPlay`
  (bind _chasmwidth (`self.ChasmWidth`))
  (bind _newchunk (`self.NewChunk`))
  (bind _chunkindex (`self.ChunkIndex`))
  (for _index (range 20)
    (bind _rowlrthickness (`self.ComputeLRThickness` _chunkindex _index _chasmwidth))
    (`KismetArrayLibrary.Array_Add` (`self.NewChunk`) _rowlrthickness))
  (`KismetArrayLibrary.Array_Add` (`self.Maps`) (make `/Game/Individual_Folders/Ryan/S_Map` _chunkindex _newchunk))
  (set `self.BoundedChunk` _newchunk)
  (bind _result (`/Engine/EditorBlueprintResources/StandardMacros.DecrementInt` (`self.ChunkIndex`))
    (:`  `
      (bind _rowlrthickness_2 (`self.ComputeLRThickness` _result 19 _chasmwidth))
      (`KismetArrayLibrary.Array_Insert` (`self.BoundedChunk`) _rowlrthickness_2)
      (bind _rowlrthickness_3 (`self.ComputeLRThickness` (`self.ChunkIndex`) 20 _chasmwidth))
      (`KismetArrayLibrary.Array_Insert` (`self.BoundedChunk`) _rowlrthickness_3 21)
      (bind _returnvalue (`|SpawnActorFromClass` "/Script/Paper2D.PaperTileMapActor" (`KismetMathLibrary.MakeTransform` (`KismetMathLibrary.MakeVector` -928.0 0.0 (`KismetMathLibrary.Conv_IntToDouble` (- (- (* (`self.ChunkIndex`) -1280) 480) 960)))) "Undefined" "OverrideRootScale" null null))
      (bind _returnvalue_2 (`AddComponent|NODE_AddPaperTileMapComponent-0` :`self` _returnvalue))
      (`PaperTileMapComponent.CreateNewTileMap` _returnvalue_2 30 20 64 64 1.0 true)
      (`self.PlaceTiles` _returnvalue_2)
      (`PrimitiveComponent.SetCollisionResponseToChannel` _returnvalue_2 "ECC_Pawn" "ECR_Block")
      (`PaperTileMapComponent.RebuildCollision` _returnvalue_2))))

(fn `ComputeLRThickness`
  (params (ChunkIndex :type Integer) (RowIndex :type Integer) (ChasmWidth :type "Float (double-precision)"))
  (returns (RowLRThickness :type "IntPoint Structure"))
  (bind _returnvalue (`KismetMathLibrary.FCeil` ChasmWidth))
  (bind _returnvalue_2 (/ ChasmWidth 2.0))
  (bind (_seeds_x _seeds_y) (break `IntPoint` (`self.Seeds`)))
  (bind _returnvalue_3 (+ (`KismetMathLibrary.Conv_IntToDouble` ChunkIndex) (/ (`KismetMathLibrary.Conv_IntToDouble` RowIndex) 20.0)))
  (bind _returnvalue_4 (* _returnvalue_3 (`self.IrregularityFrequency`)))
  (bind _returnvalue_5 (`KismetMathLibrary.Clamp` (+ (- 15 (+ (`KismetMathLibrary.FFloor` (* (`KismetMathLibrary.PerlinNoise1D` (* (+ (`KismetMathLibrary.Conv_IntToDouble` _seeds_x) _returnvalue_3) (`self.ChasmFrequency`))) (- 14.0 _returnvalue_2))) (`KismetMathLibrary.FCeil` _returnvalue_2))) (`KismetMathLibrary.FFloor` (* _returnvalue (* (`KismetMathLibrary.PerlinNoise1D` (+ _returnvalue_4 (`KismetMathLibrary.Conv_IntToDouble` _seeds_x))) (`self.IrregularityScale`))))) 1 (- 30 (+ _returnvalue 1))))
  (bind _returnvalue_6 (- (- 30 _returnvalue_5) _returnvalue))
  (return (make `IntPoint` _returnvalue_5 (`KismetMathLibrary.Clamp` (+ _returnvalue_6 (`KismetMathLibrary.FFloor` (* _returnvalue (* (`KismetMathLibrary.PerlinNoise1D` (+ _returnvalue_4 (`KismetMathLibrary.Conv_IntToDouble` _seeds_y))) (`self.IrregularityScale`))))) 1 (`KismetMathLibrary.Clamp` (- _returnvalue_6 2) 1 30)))))

(fn `DetermineTile`
  (params (TileInteger :type Integer) (RowLength :type Integer) (RowLengthAbove :type Integer) (RowLengthBelow :type Integer) (`isLeftSide?` :type Boolean))
  (returns (TilesetInteger :type Integer))
  (locals (ChosenTile :type Integer))
  (bind _returnvalue (>= TileInteger RowLengthAbove))
  (bind _returnvalue_2 (>= TileInteger RowLengthAbove))
  (bind _returnvalue_3 (== TileInteger (- RowLengthAbove 1)))
  (bind _returnvalue_4 (== TileInteger (- RowLengthBelow 1)))
  (bind _returnvalue_5 (== TileInteger (- RowLengthBelow 1)))
  (bind _returnvalue_6 (== TileInteger (- RowLengthAbove 1)))
  (if `isLeftSide?`
    (if (== TileInteger RowLength)
      (if (and (< TileInteger RowLengthAbove) (< TileInteger RowLengthBelow))
        (set `local.ChosenTile` 23)
        (elif (< TileInteger RowLengthAbove)
          (set `local.ChosenTile` 17)
          (elif (< TileInteger RowLengthBelow)
            (set `local.ChosenTile` 8)
            (else
              (set `local.ChosenTile` 5)))))
      (elif (and (< TileInteger (- RowLengthAbove 1)) (< TileInteger (- RowLengthBelow 1)))
        (set `local.ChosenTile` 24)
        (elif (and _returnvalue_3 _returnvalue_4)
          (set `local.ChosenTile` 29)
          (elif _returnvalue_3
            (if (>= TileInteger RowLengthBelow)
              (set `local.ChosenTile` 50)
              (else
                (set `local.ChosenTile` 27)))
            (elif _returnvalue_4
              (if (>= TileInteger RowLengthAbove)
                (set `local.ChosenTile` 41)
                (else
                  (set `local.ChosenTile` 18)))
              (elif (and (>= TileInteger RowLengthBelow) _returnvalue)
                (set `local.ChosenTile` 2)
                (elif _returnvalue
                  (set `local.ChosenTile` 31)
                  (elif (not _returnvalue)
                    (set `local.ChosenTile` 32)
                    (else
                      (set `local.ChosenTile` 35 :!label _label))))))))))
    (elif (== TileInteger RowLength)
      (if (and (< TileInteger RowLengthAbove) (< TileInteger RowLengthBelow))
        (set `local.ChosenTile` 22)
        (elif (< TileInteger RowLengthAbove)
          (set `local.ChosenTile` 16)
          (elif (< TileInteger RowLengthBelow)
            (set `local.ChosenTile` 7)
            (else
              (set `local.ChosenTile` 15)))))
      (elif (and (< TileInteger (- RowLengthAbove 1)) (< TileInteger (- RowLengthBelow 1)))
        (set `local.ChosenTile` 24)
        (elif (and _returnvalue_6 _returnvalue_5)
          (set `local.ChosenTile` 30)
          (elif _returnvalue_6
            (if (>= TileInteger RowLengthBelow)
              (set `local.ChosenTile` 49)
              (else
                (set `local.ChosenTile` 28)))
            (elif _returnvalue_5
              (if (>= TileInteger RowLengthAbove)
                (set `local.ChosenTile` 40)
                (else
                  (set `local.ChosenTile` 19)))
              (elif (and (>= TileInteger RowLengthBelow) _returnvalue_2)
                (set `local.ChosenTile` 2)
                (elif _returnvalue_2
                  (set `local.ChosenTile` 31)
                  (elif (not _returnvalue_2)
                    (set `local.ChosenTile` 32)
                    (else
                      (goto _label)))))))))))
  (return (`local.ChosenTile`)))

(fn `PlaceTiles`
  (params (Tilemap :type "PaperTileMapComponent Object Reference"))
  (bind _boundedchunk (`self.BoundedChunk`))
  (for (_array_element _array_index) (`self.NewChunk`)
    (bind (_x _y) (break `IntPoint` _array_element))
    (bind _returnvalue (- _x 1))
    (for _index (range (+ _returnvalue 1))
      (bind (_output_x _output_y) (break `IntPoint` (`|GetArrayItem` _boundedchunk _array_index)))
      (bind (_output_x_2 _output_y_2) (break `IntPoint` (`|GetArrayItem` _boundedchunk (+ _array_index 2))))
      (bind _tilesetinteger (`self.DetermineTile` _index _returnvalue _output_x _output_x_2 true))
      (`PaperTileMapComponent.SetTile` Tilemap _index _array_index 0 (`TileMapBlueprintLibrary.MakeTile` _tilesetinteger "/Game/COP26/Art/Tilemaps/Placeholder/Placeholder_Tiles_TileSet.Placeholder_Tiles_TileSet")))
    (bind _returnvalue_2 (- _y 1))
    (for _index_2 (range (+ _returnvalue_2 1))
      (bind _tilesetinteger_2 (`self.DetermineTile` _index_2 _returnvalue_2 _output_y _output_y_2))
      (`PaperTileMapComponent.SetTile` Tilemap (- 29 _index_2) _array_index 0 (`TileMapBlueprintLibrary.MakeTile` _tilesetinteger_2 "/Game/COP26/Art/Tilemaps/Placeholder/Placeholder_Tiles_TileSet.Placeholder_Tiles_TileSet"))
      (`PaperTileMapComponent.SetTile` Tilemap (- 29 _index_2) _array_index 0 (`TileMapBlueprintLibrary.MakeTile` _tilesetinteger_2 "/Game/COP26/Art/Tilemaps/Placeholder/Placeholder_Tiles_TileSet.Placeholder_Tiles_TileSet")))))

(fn `UserConstructionScript`)